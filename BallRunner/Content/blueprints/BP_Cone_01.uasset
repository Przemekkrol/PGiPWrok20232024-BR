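; BP_Cone_01 is a collectible-style actor with a point light that reacts when the player pawn overlaps its trigger.
; On overlap it plays a frog laugh meme sound, waits briefly, then runs a timeline.
; Each timeline update lerps from the current location, scale and light intensity toward the player, zero size and darkness, then the actor destroys itself when finished.
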(event OnComponentBeginOverlap(trigger)
  (params (OverlappedComponent :type Primitive%20Component%20Object%20Reference) (OtherActor :type Actor%20Object%20Reference) (OtherComp :type Primitive%20Component%20Object%20Reference) (OtherBodyIndex :type Integer) (bFromSweep :type Boolean) (SweepResult :type Hit%20Result%20Structure%20%28by%20ref%29))
  (bind _pointlight (Variables|Default|GetPointLight))
  (if (== OtherActor (Game|Player|GetPlayerPawn 0))
    (Audio|SpawnSound2D "/Game/blueprints/Frog_Meme_Laugh__TikTok_sound_effect.Frog_Meme_Laugh__TikTok_sound_effect" 1.0 1.0 0.0 0)
    (Utilities|FlowControl|Delay 0.2)
    (bind (_direction _crystalmovement _crystalscale _newtrack_2) (Timeline|Timeline_0 Play)
      (:Update
        (Transformation|SetActorLocation (Math|Vector|Lerp(Vector) (Transformation|GetActorLocation) (Transformation|GetActorLocation (Game|Player|GetPlayerPawn 0)) _crystalmovement) false false)
        (Transformation|SetActorScale3D (Math|Vector|Lerp(Vector) (Transformation|GetActorScale3D) "0, 0, 0" _crystalscale))
        (Rendering|Components|Light|SetIntensity _pointlight (Math|Float|Lerp (Variables|/Script/Engine.LightComponentBase|GetIntensity _pointlight) 0.0 _newtrack_2)))
      (:Finished
        (Actor|DestroyActor)))))

(fn ConstructionScript)