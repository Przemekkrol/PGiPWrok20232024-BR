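; Player-controlled ball Blueprint that rolls by physics torque and restarts the current level when damaged.
; ForwardBack and LeftRight axis inputs apply acceleration-change torque to the Sphere, scaled by the ForceMultiply variable and a hardcoded factor respectively.
; Any damage fires once, starting a zero-length camera fade and zero delay before reopening the level by name.
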(event Game|Damage|EventAnyDamage
  (params (Damage :type Float%20%28single-precision%29) (DamageType :type Damage%20Type%20Object%20Reference) (InstigatedBy :type Controller%20Object%20Reference) (DamageCauser :type Actor%20Object%20Reference))
  (bind _returnvalue (Math|Float|MakeLiteralFloat 0.0))
  (Utilities|FlowControl|DoOnce false
    (:Completed
      (CameraFades|StartCameraFade :self (Game|GetPlayerCameraManager 0) :Duration _returnvalue)
      (Utilities|FlowControl|Delay _returnvalue)
      (bind _returnvalue_2 (Game|GetCurrentLevelName true))
      (Game|OpenLevel(byName) (Utilities|String|StringToName _returnvalue_2)))))

(event Input|AxisEvents|InputAxisForwardBack
  (params (AxisValue :type Float%20%28single-precision%29))
  ;[1 1 1] ball movement torque
  (Class|PrimitiveComponent|AddTorqueinRadians (Variables|Default|GetSphere) (Math|Vector|MakeVector 0.0 (* AxisValue (Variables|Default|GetForceMultiply)) 0.0) "None" true))

(event Input|AxisEvents|InputAxisLeftRight
  (params (AxisValue :type Float%20%28single-precision%29))
  ;[1 1 1] ball movement torque
  (Class|PrimitiveComponent|AddTorqueinRadians (Variables|Default|GetSphere) (Math|Vector|MakeVector (* AxisValue -17.0) 0.0 0.0) "None" true))

(fn ConstructionScript)