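; Level-exit trigger volume that completes the level when the player pawn enters it with no BP_Crystal actors left in the world.
; If crystals remain, it prints a Polish message telling the player to collect the rest.
; Completion finds the current level in an ordered LevelNames array and opens the next entry, or quits the game on the last one.
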(event OnComponentBeginOverlap(WinVolume)
  (params (OverlappedComponent :type Primitive%20Component%20Object%20Reference) (OtherActor :type Actor%20Object%20Reference) (OtherComp :type Primitive%20Component%20Object%20Reference) (OtherBodyIndex :type Integer) (bFromSweep :type Boolean) (SweepResult :type Hit%20Result%20Structure%20%28by%20ref%29))
  (if (== OtherActor (Game|Player|GetPlayerPawn 0))
    (bind _outactors (Actor|GetAllActorsOfClass "/Game/blueprints/BP_Crystal.BP_Crystal_C"))
    (if (> (Utilities|Array|Length _outactors) 0)
      (Development|PrintString "Zbierz pozostałe kryształki")
      (else
        (LevelManagement|CompleteLevel)))))

(fn ConstructionScript)

(fn GetCurrentLevelIndex
  (bind _returnvalue (Game|GetCurrentLevelName true))
  (return (Utilities|Array|FindItem (Variables|Default|GetLevelNames) (Utilities|String|StringToName _returnvalue))))

(fn CompleteLevel
  (if (LevelManagement|IsFinalLevel)
    (Game|QuitGame 0 "Quit" false)
    (else
      (LevelManagement|LoadNewLevel))))

(fn IsFinalLevel
  (return (== (Utilities|Array|LastIndex (Variables|Default|GetLevelNames)) (LevelManagement|GetCurrentLevelIndex))))

(fn LoadNewLevel
  (Game|OpenLevel(byName) (LevelManagement|GetNextLevelName)))

(fn GetNextLevelName
  (return (Utilities|Array|Get(acopy) (Variables|Default|GetLevelNames) (+ (LevelManagement|GetCurrentLevelIndex) 1))))